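; Paper2D fighter character shared by both players in a local two-player versus game, with player two tinted by the construction script.
; Enhanced Input drives movement along X, jumping and pause, while player-two inputs are forwarded to pawn 1.
; Attacks jump to ground or air animation nodes, with separate events damaging actors overlapping hit boxes.
; Damage updates health and briefly halts walking; death disables both players and calls the winner check.
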(event `EnhancedInput|/Game/Controls/EA_PauseGame`
  (params (ActionValue :type Boolean) (ElapsedSeconds :type "Float (double-precision)") (TriggeredSeconds :type "Float (double-precision)") (InputAction :type "InputAction Object Reference" :default "/Game/Controls/EA_PauseGame.EA_PauseGame"))
  (bind _returnvalue (`GameplayStatics.GetPlayerController` 0))
  (:`Completed`
    (if (not (`self.IsPauseMenuOpen`))
      (set `self.IsPauseMenuOpen` true)
      (bind _returnvalue_2 (`|CreateWidget` "/Game/Menus/PauseMenu/PauseMenu.PauseMenu_C" _returnvalue))
      (bind _output_get (set `self.PauseMenuWidget` _returnvalue_2))
      (`UserWidget.AddToViewport` _output_get 0)
      (`WidgetBlueprintLibrary.SetInputMode_GameAndUIEx` _returnvalue (`self.PauseMenuWidget`))
      (set `PlayerController.bShowMouseCursor` true (`GameplayStatics.GetPlayerController` 0))
      (`GameplayStatics.SetGamePaused` true)
      (`KismetSystemLibrary.Delay` 2.0)
      (else
        (set `self.IsPauseMenuOpen` false)
        (`Widget.RemoveFromParent` (`self.PauseMenuWidget`))
        (`GameplayStatics.SetGamePaused` false)
        (`WidgetBlueprintLibrary.SetInputMode_GameOnly` _returnvalue)
        (set `PlayerController.bShowMouseCursor` false (`GameplayStatics.GetPlayerController` 0))))))

(event `LoadControls`
  (bind _asplayer_controller (cast `PlayerController` (`self.GetController`) :!label _label))
  (bind _returnvalue (pcsubsystem `EnhancedInputLocalPlayerSubsystem` _asplayer_controller))
  (`/Engine/EditorBlueprintResources/StandardMacros.IsValid` _returnvalue
    (:`Is Valid`
      (`EnhancedInputSubsystemInterface.AddMappingContext` _returnvalue "/Game/Controls/Fighting_IMC.Fighting_IMC" 0 (struct))
      (set `self.PlayerSpeed` (`CharacterMovementComponent.MaxWalkSpeed` (`self.CharacterMovement`)))
      (set `self.PlayerMaxHealth` (`self.Playerhealth`)))))

(event `self.ReceiveBeginPlay`
  (goto _label))

(event `Player2Jump`
  (`self.Jump` :!label _label_2))

(event `AirAttack`
  ;[1 1 1] AirAttack
  (for _array_element (`PrimitiveComponent.GetOverlappingActors` (`self.AirBox`) null)
    (if (!= _array_element self)
      (`GameplayStatics.ApplyDamage` _array_element (`self.Base Damage`)))))

(event `EnhancedInput|/Game/Controls/Jump_IA`
  (params (ActionValue :type Boolean) (ElapsedSeconds :type "Float (double-precision)") (TriggeredSeconds :type "Float (double-precision)") (InputAction :type "InputAction Object Reference" :default "/Game/Controls/Jump_IA.Jump_IA"))
  (:`Started`
    (goto _label_2))
  (:`Canceled`
    (`self.StopJumping`)))

(event `Attack`
  ;[1 1 1] Attack
  (for _array_element (`PrimitiveComponent.GetOverlappingActors` (`self.AttackBox`) null)
    (if (!= _array_element self)
      (`GameplayStatics.ApplyDamage` _array_element (`self.Base Damage`)))))

(event `EnhancedInput|/Game/Controls/Move_IA`
  (params (ActionValue :type "Float (double-precision)") (ElapsedSeconds :type "Float (double-precision)") (TriggeredSeconds :type "Float (double-precision)") (InputAction :type "InputAction Object Reference" :default "/Game/Controls/Move_IA.Move_IA"))
  ;[1 1 1] Attack System
  (:`Triggered`
    (`self.AddMovementInput` (1.0 0.0 0.0) ActionValue)))

(event `Player2Attack`
  ;[1 1 1] Attack System
  (`/Engine/EditorBlueprintResources/StandardMacros.DoOnce` false :!label _label_3
    (:`Completed`
      (set `CharacterMovementComponent.MaxWalkSpeed` 0.0 (`self.CharacterMovement`))
      (if (`NavMovementComponent.IsFalling` (`self.CharacterMovement`))
        ;;[1 1 1] AirAttack
        (`PaperZDAnimInstance.JumpToNode` (`PaperZDAnimationComponent.AnimInstance` (`self.AnimationComponent`)) "AirAttack" "None")
        (`KismetSystemLibrary.Delay` (`PaperFlipbookComponent.GetFlipbookLength` (`self.Sprite`)))
        (else
          ;;[1 1 1] GroundAttack
          (`PaperZDAnimInstance.JumpToNode` (`PaperZDAnimationComponent.AnimInstance` (`self.AnimationComponent`)) "Attack" "None")
          (`KismetSystemLibrary.Delay` (`PaperFlipbookComponent.GetFlipbookLength` (`self.Sprite`)))))
      (set `CharacterMovementComponent.MaxWalkSpeed` (`self.PlayerSpeed`) (`self.CharacterMovement`))
      (goto _label_3 :!via `Reset`))))

(event `self.ReceiveAnyDamage`
  (params (Damage :type "Float (single-precision)") (DamageType :type "DamageType Object Reference") (InstigatedBy :type "Controller Object Reference") (DamageCauser :type "Actor Object Reference"))
  (bind _output_get (set `self.Playerhealth` (- (`self.Playerhealth`) Damage)))
  (`self.Updatehealth`)
  (if (<= _output_get 0.0)
    (`/Engine/EditorBlueprintResources/StandardMacros.DoOnce` false
      (:`Completed`
        (`PaperZDAnimInstance.JumpToNode` (`PaperZDAnimationComponent.AnimInstance` (`self.AnimationComponent`)) "Death" "None")
        (`self.DisableInput` (`GameplayStatics.GetPlayerPawn` 0) null)
        (`self.DisableInput` (`GameplayStatics.GetPlayerPawn` 1) null)
        (`self.WhoWon`)))
    (else
      (`PaperZDAnimInstance.JumpToNode` (`PaperZDAnimationComponent.AnimInstance` (`self.AnimationComponent`)) "damaged" "None")
      (set `CharacterMovementComponent.MaxWalkSpeed` 0.0 (`self.CharacterMovement`))
      (`KismetSystemLibrary.RetriggerableDelay` (`PaperFlipbookComponent.GetFlipbookLength` (`self.Sprite`)))
      (set `CharacterMovementComponent.MaxWalkSpeed` (`self.PlayerSpeed`) (`self.CharacterMovement`)))))

(event `EnhancedInput|/Game/Controls/Attack_IA`
  (params (ActionValue :type Boolean) (ElapsedSeconds :type "Float (double-precision)") (TriggeredSeconds :type "Float (double-precision)") (InputAction :type "InputAction Object Reference" :default "/Game/Controls/Attack_IA.Attack_IA"))
  ;[1 1 1] Attack System
  (:`Started`
    (goto _label_3)))

(event `MovePlayer2`
  (params (axisvalue :type "Float (double-precision)"))
  ;[1 1 1] MovePlayer2
  (`self.AddMovementInput` (1.0 0.0 0.0) axisvalue))

(event `EnhancedInput|/Game/Controls/MovePlayer2_IA`
  (params (ActionValue :type "Float (double-precision)") (ElapsedSeconds :type "Float (double-precision)") (TriggeredSeconds :type "Float (double-precision)") (InputAction :type "InputAction Object Reference" :default "/Game/Controls/MovePlayer2_IA.MovePlayer2_IA"))
  (bind _player2 (`self.player2`))
  ;[1 1 1] MovePlayer2
  (:`Triggered`
    (`/Engine/EditorBlueprintResources/StandardMacros.IsValid` _player2
      (:`Is Valid`
        (`self.MovePlayer2` _player2 ActionValue))
      (:`Is Not Valid`
        (bind _asplayer_character_bp (cast `/Game/Blueprints/Character_BPs/PlayerCharacter_BP` (`GameplayStatics.GetPlayerPawn` 1)))
        (bind _output_get (set `self.player2` _asplayer_character_bp))
        (`self.MovePlayer2` _output_get ActionValue)))))

(event `Key|Up`
  (params (Key :type "Key Structure"))
  (bind _player2 (`self.player2`))
  ;[1 1 1] MovePlayer2
  (:`Pressed`
    (`/Engine/EditorBlueprintResources/StandardMacros.IsValid` _player2
      (:`Is Valid`
        (`self.Player2Jump` _player2))
      (:`Is Not Valid`
        (bind _asplayer_character_bp (cast `/Game/Blueprints/Character_BPs/PlayerCharacter_BP` (`GameplayStatics.GetPlayerPawn` 1)))
        (bind _output_get (set `self.player2` _asplayer_character_bp))
        (`self.Player2Jump` _output_get)))))

(event `Key|Down`
  (params (Key :type "Key Structure"))
  (bind _player2 (`self.player2`))
  ;[1 1 1] MovePlayer2
  (:`Pressed`
    (`/Engine/EditorBlueprintResources/StandardMacros.IsValid` _player2
      (:`Is Valid`
        (`self.Player2Attack` _player2))
      (:`Is Not Valid`
        (bind _asplayer_character_bp (cast `/Game/Blueprints/Character_BPs/PlayerCharacter_BP` (`GameplayStatics.GetPlayerPawn` 1)))
        (bind _output_get (set `self.player2` _asplayer_character_bp))
        (`self.Player2Attack` _output_get)))))

(fn `UserConstructionScript`
  (if (`self.isplayer2`)
    (`PaperFlipbookComponent.SetSpriteColor` (`self.Sprite`) (struct :`R` 1.0 :`G` 0.378811 :`B` 0.25 :`A` 1.0))))