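; Player character for a two-player local 2D fighter, with single-axis movement, jumping, a health bar widget and ground or air attacks.
; Enhanced Input drives the pawn and also relays Player 2's move, jump and attack to the cached pawn at player index 1, which is tinted when flagged.
; Attacks jump to PaperZD animation nodes, gated by a DoOnce that resets after the flipbook length.
; The F key applies test damage.
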(event `Key|F`
  (params (Key :type "Key Structure"))
  (:`Pressed`
    (bind _output_get (set `self.health` (`KismetMathLibrary.FClamp` (- (`self.health`) 10.0) 0.0 100.0)))
    (`KismetSystemLibrary.PrintString` (`KismetStringLibrary.Conv_DoubleToString` _output_get))))

(event `LoadControls`
  (bind _asplayer_controller (cast `PlayerController` (`self.GetController`) :!label _label))
  (bind _returnvalue (pcsubsystem `EnhancedInputLocalPlayerSubsystem` _asplayer_controller))
  (`/Engine/EditorBlueprintResources/StandardMacros.IsValid` _returnvalue
    (:`Is Valid`
      (`EnhancedInputSubsystemInterface.AddMappingContext` _returnvalue "/Game/Controls/Fighting_IMC.Fighting_IMC" 0 (struct)))))

(event `self.ReceiveBeginPlay`
  (bind _returnvalue (`|CreateWidget` "/Game/HealthItems/HealthBar.HealthBar_C"))
  (`UserWidget.AddToViewport` _returnvalue 0)
  (goto _label))

(event `Player2Jump`
  (`self.Jump` :!label _label_2))

(event `EnhancedInput|/Game/Controls/Jump_IA`
  (params (ActionValue :type Boolean) (ElapsedSeconds :type "Float (double-precision)") (TriggeredSeconds :type "Float (double-precision)") (InputAction :type "InputAction Object Reference" :default "/Game/Controls/Jump_IA.Jump_IA"))
  (:`Started`
    (goto _label_2))
  (:`Canceled`
    (`self.StopJumping`)))

(event `EnhancedInput|/Game/Controls/Move_IA`
  (params (ActionValue :type "Float (double-precision)") (ElapsedSeconds :type "Float (double-precision)") (TriggeredSeconds :type "Float (double-precision)") (InputAction :type "InputAction Object Reference" :default "/Game/Controls/Move_IA.Move_IA"))
  ;[1 1 1] Attack System
  (:`Triggered`
    (`self.AddMovementInput` (1.0 0.0 0.0) ActionValue)))

(event `Player2Attack`
  ;[1 1 1] Attack System
  (`/Engine/EditorBlueprintResources/StandardMacros.DoOnce` false :!label _label_3
    (:`Completed`
      (if (`NavMovementComponent.IsFalling` (`self.CharacterMovement`))
        ;;[1 1 1] AirAttack
        (`PaperZDAnimInstance.JumpToNode` (`PaperZDAnimationComponent.AnimInstance` (`self.AnimationComponent`)) "AirAttack" "None")
        (`KismetSystemLibrary.Delay` (`PaperFlipbookComponent.GetFlipbookLength` (`self.Sprite`)))
        (goto _label_3 :!via `Reset`)
        (else
          ;;[1 1 1] GroundAttack
          (`PaperZDAnimInstance.JumpToNode` (`PaperZDAnimationComponent.AnimInstance` (`self.AnimationComponent`)) "Attack" "None")
          (`KismetSystemLibrary.Delay` (`PaperFlipbookComponent.GetFlipbookLength` (`self.Sprite`)))
          (goto _label_3 :!via `Reset`))))))

(event `EnhancedInput|/Game/Controls/Attack_IA`
  (params (ActionValue :type Boolean) (ElapsedSeconds :type "Float (double-precision)") (TriggeredSeconds :type "Float (double-precision)") (InputAction :type "InputAction Object Reference" :default "/Game/Controls/Attack_IA.Attack_IA"))
  ;[1 1 1] Attack System
  (:`Started`
    (goto _label_3)))

(event `MovePlayer2`
  (params (axisvalue :type "Float (double-precision)"))
  ;[1 1 1] MovePlayer2
  (`self.AddMovementInput` (1.0 0.0 0.0) axisvalue))

(event `EnhancedInput|/Game/Controls/MovePlayer2_IA`
  (params (ActionValue :type "Float (double-precision)") (ElapsedSeconds :type "Float (double-precision)") (TriggeredSeconds :type "Float (double-precision)") (InputAction :type "InputAction Object Reference" :default "/Game/Controls/MovePlayer2_IA.MovePlayer2_IA"))
  (bind _player2 (`self.player2`))
  ;[1 1 1] MovePlayer2
  (:`Triggered`
    (`/Engine/EditorBlueprintResources/StandardMacros.IsValid` _player2
      (:`Is Valid`
        (`self.MovePlayer2` _player2 ActionValue))
      (:`Is Not Valid`
        (bind _asplayer_character_bp (cast `/Game/Characters/Monk/Blueprint/PlayerCharacter_BP` (`GameplayStatics.GetPlayerPawn` 1)))
        (bind _output_get (set `self.player2` _asplayer_character_bp))
        (`self.MovePlayer2` _output_get ActionValue)))))

(event `Key|Up`
  (params (Key :type "Key Structure"))
  (bind _player2 (`self.player2`))
  ;[1 1 1] MovePlayer2
  (:`Pressed`
    (`/Engine/EditorBlueprintResources/StandardMacros.IsValid` _player2
      (:`Is Valid`
        (`self.Player2Jump` _player2))
      (:`Is Not Valid`
        (bind _asplayer_character_bp (cast `/Game/Characters/Monk/Blueprint/PlayerCharacter_BP` (`GameplayStatics.GetPlayerPawn` 1)))
        (bind _output_get (set `self.player2` _asplayer_character_bp))
        (`self.Player2Jump` _output_get)))))

(event `Key|Down`
  (params (Key :type "Key Structure"))
  (bind _player2 (`self.player2`))
  ;[1 1 1] MovePlayer2
  (:`Pressed`
    (`/Engine/EditorBlueprintResources/StandardMacros.IsValid` _player2
      (:`Is Valid`
        (`self.Player2Attack` _player2))
      (:`Is Not Valid`
        (bind _asplayer_character_bp (cast `/Game/Characters/Monk/Blueprint/PlayerCharacter_BP` (`GameplayStatics.GetPlayerPawn` 1)))
        (bind _output_get (set `self.player2` _asplayer_character_bp))
        (`self.Player2Attack` _output_get)))))

(fn `UserConstructionScript`
  (if (`self.isplayer2`)
    (`PaperFlipbookComponent.SetSpriteColor` (`self.Sprite`) (struct :`R` 1.0 :`G` 0.378811 :`B` 0.25 :`A` 1.0))))