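; Side-scrolling skeleton enemy that patrols along the X axis, attacks the player and takes damage.
; Tick drives movement and facing, with forward and downward traces triggering a pause and turnaround at obstacles or ledges.
; A box overlap halts patrol and loops a timed attack animation, while a separate Attack event traces to damage the player.
; Damage updates the health bar widget, then knocks the skeleton back or plays death and destroys it.
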(event `self.ReceiveBeginPlay`
  ;[1 1 1] Event begin play
  (set `CharacterMovementComponent.MaxWalkSpeed` (`self.Max Walk Speed`) (`self.CharacterMovement`))
  (set `self.maxhealth` (`self.health`))
  (bind _asenemy_health_bar_wb (cast `` (`WidgetComponent.GetWidget` (`self.Widget`))))
  (set `/Game/Skeleton/blueprints/Skeleton_BP.skeletonref` self _asenemy_health_bar_wb)
  (set `self.As Enemy Health Bar WB` null _asenemy_health_bar_wb))

(event `self.ReceiveTick`
  (params (DeltaSeconds :type "Float (single-precision)"))
  ;[1 1 1] Event tick
  (`self.Handle rotation`)
  (`self.Handlemovement`))

(event `Handlemovement`
  (bind _returnvalue (`self.K2_GetActorLocation`))
  (bind _returnvalue_2 (`self.K2_GetActorLocation`))
  ;[1 1 1] Handle movement
  (if (not (or (`self.isdead`) (`self.enemydamaged`) (`NavMovementComponent.IsFalling` (`self.CharacterMovement`)) (`self.attackmode`)))
    (`self.AddMovementInput` (1.0 0.0 0.0) (`self.movementdirection`))
    (`|ExecutionSequence`
      (:`then_0`
        ;;[1 1 1] Detect if object is in front of skeleton
        (bind (_outhit _returnvalue_3) (`KismetSystemLibrary.LineTraceSingleForObjects` _returnvalue_2 (+ _returnvalue_2 (* (`self.GetActorForwardVector`) (100.0 0.0 0.0))) (`|MakeArray` "ObjectTypeQuery1" "ObjectTypeQuery2" "ObjectTypeQuery3" :!type "EObjectTypeQuery Enum") false (`|MakeArray` (`GameplayStatics.GetPlayerCharacter` 0) :!type "Actor Object Reference")))
        (if _returnvalue_3
          (`/Engine/EditorBlueprintResources/StandardMacros.DoOnce` false :!label _label
            (:`Completed`
              (set `CharacterMovementComponent.MaxWalkSpeed` 0.0 (`self.CharacterMovement`))
              (`KismetSystemLibrary.Delay` (`self.waittime`))
              (set `CharacterMovementComponent.MaxWalkSpeed` (`self.Max Walk Speed`) (`self.CharacterMovement`))
              (set `self.movementdirection` (* (`self.movementdirection`) -1.0))
              (goto _label :!via `Reset`)))))
      (:`then_1`
        ;;[1 1 1] detect if skeleton is on edge of world
        (bind (_outhit_2 _returnvalue_4) (`KismetSystemLibrary.LineTraceSingleForObjects` _returnvalue (+ (- _returnvalue (0.0 0.0 100.0)) (* (`self.GetActorForwardVector`) (100.0 0.0 0.0))) (`|MakeArray` "ObjectTypeQuery1" "ObjectTypeQuery2" "ObjectTypeQuery3" :!type "EObjectTypeQuery Enum") false (`|MakeArray` (`GameplayStatics.GetPlayerCharacter` 0) :!type "Actor Object Reference")))
        (if (not _returnvalue_4)
          (goto _label))))))

(event `Handle rotation`
  ;[1 1 1] Handle rotation
  (if (`self.isdead`)
    _
    (elif (> (`self.movementdirection`) 0.0)
      (`self.K2_SetActorRotation` (struct))
      (else
        (`self.K2_SetActorRotation` (struct :`Yaw` 180.0))))))

(event `self.Box.OnComponentBeginOverlap`
  (params (OverlappedComponent :type "PrimitiveComponent Object Reference") (OtherActor :type "Actor Object Reference") (OtherComp :type "PrimitiveComponent Object Reference") (OtherBodyIndex :type Integer) (bFromSweep :type Boolean) (SweepResult :type "HitResult Structure (by ref)"))
  ;[1 1 1] Handle attack system
  (if (== OtherActor (`GameplayStatics.GetPlayerCharacter` 0))
    (set `self.attackmode` true)
    (bind _returnvalue (`KismetSystemLibrary.K2_SetTimerDelegate` (delegate `skeletonattack`) 1.0 true))
    (set `self.attackevent` _returnvalue)))

(event `skeletonattack`
  ;[1 1 1] Handle attack system
  (if (not (`self.isdead`))
    (`PaperZDAnimInstance.JumpToNode` (`PaperZDAnimationComponent.AnimInstance` (`self.AnimationComponent`)) (`self.attackjumpnode`) "None")))

(event `self.Box.OnComponentEndOverlap`
  (params (OverlappedComponent :type "PrimitiveComponent Object Reference") (OtherActor :type "Actor Object Reference") (OtherComp :type "PrimitiveComponent Object Reference") (OtherBodyIndex :type Integer))
  ;[1 1 1] Handle attack system
  (if (== OtherActor (`GameplayStatics.GetPlayerCharacter` 0))
    (set `self.attackmode` false)
    (`KismetSystemLibrary.K2_ClearAndInvalidateTimerHandle` (`self.attackevent`))))

(event `self.ReceiveAnyDamage`
  (params (Damage :type "Float (single-precision)") (DamageType :type "DamageType Object Reference") (InstigatedBy :type "Controller Object Reference") (DamageCauser :type "Actor Object Reference"))
  (bind _returnvalue_x (`KismetMathLibrary.BreakVector` (`KismetMathLibrary.GetDirectionUnitVector` (`self.K2_GetActorLocation` DamageCauser) (`self.K2_GetActorLocation`))))
  (bind _returnvalue (select `bool` (< _returnvalue_x 0.0) :`false` -1.0 :`true` 1.0))
  ;[1 1 1] Handle damage
  (set `self.health` (- (`self.health`) Damage))
  (`self.Updatehealthbar` (`.As Enemy Health Bar WB` (`self.As Enemy Health Bar WB`)))
  (set `self.enemydamaged` true)
  (set `self.movementdirection` _returnvalue)
  (if (<= (`self.health`) 0.0)
    (`PaperZDAnimInstance.JumpToNode` (`PaperZDAnimationComponent.AnimInstance` (`self.AnimationComponent`)) (`self.deathjumpnode`) "None")
    (set `self.isdead` true)
    (`SceneComponent.SetVisibility` (`self.Widget`) false false)
    (`PrimitiveComponent.SetCollisionProfileName` (`self.CapsuleComponent`) "OverlapOnlyPawn" true)
    (`KismetSystemLibrary.Delay` 3.0)
    (`self.K2_DestroyActor`)
    (else
      (`self.LaunchCharacter` (`KismetMathLibrary.MakeVector` (* _returnvalue -1200.0) 0.0 300.0) true true)
      (`PaperZDAnimInstance.JumpToNode` (`PaperZDAnimationComponent.AnimInstance` (`self.AnimationComponent`)) (`self.damagedjumpnode`) "None")
      (`SceneComponent.SetVisibility` (`self.Widget`) true false)
      (`KismetSystemLibrary.RetriggerableDelay` 1.0)
      (set `self.enemydamaged` false))))

(event `Attack`
  (bind _returnvalue (`self.K2_GetActorLocation`))
  ;[1 1 1] Handle attack system
  (bind _outhit (`KismetSystemLibrary.LineTraceSingleForObjects` _returnvalue (+ _returnvalue (* (`self.GetActorForwardVector`) (100.0 0.0 0.0))) (`|MakeArray` "ObjectTypeQuery3" :!type "EObjectTypeQuery Enum")))
  (bind (_bblockinghit _binitialoverlap _time _distance _location _impactpoint _normal _impactnormal _physmat _hitactor) (`GameplayStatics.BreakHitResult` _outhit))
  (if (== _hitactor (`GameplayStatics.GetPlayerCharacter` 0))
    (`GameplayStatics.ApplyDamage` _hitactor 1.0)))

(fn `UserConstructionScript`)